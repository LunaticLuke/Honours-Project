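; BP_Door is a swinging door actor that opens and closes when the player triggers it nearby.
; BoxCollision overlap events set a NearDoor flag, which gates the Door_Open event.
; A FlipFlop alternates between playing and reversing the DoorOpenAmount timeline, whose curve scales DoorRotationAmount to drive the yaw of the SMDoor mesh.
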(event `self.BoxCollision.OnComponentBeginOverlap`
  (params (OverlappedComponent :type "PrimitiveComponent Object Reference") (OtherActor :type "Actor Object Reference") (OtherComp :type "PrimitiveComponent Object Reference") (OtherBodyIndex :type Integer) (bFromSweep :type Boolean) (SweepResult :type "HitResult Structure (by ref)"))
  ;[1 1 1] Door Detection
  (set `self.NearDoor` true))

(event `self.BoxCollision.OnComponentEndOverlap`
  (params (OverlappedComponent :type "PrimitiveComponent Object Reference") (OtherActor :type "Actor Object Reference") (OtherComp :type "PrimitiveComponent Object Reference") (OtherBodyIndex :type Integer))
  ;[1 1 1] Door Detection
  (set `self.NearDoor` false))

(event `Door_Open`
  ;[1 1 1] Door Open Sequence
  (if (`self.NearDoor`)
    (`/Engine/EditorBlueprintResources/StandardMacros.FlipFlop`
      (:`A`
        (bind (_direction _doorrotationamount) (`Timeline|DoorOpenAmount` :!label _label)
          (:`Update`
            (`SceneComponent.K2_SetRelativeRotation` (`self.SM_Door`) (`KismetMathLibrary.MakeRotator` 0.0 0.0 (* _doorrotationamount (`self.DoorRotationAmount`))) false false))))
      (:`B`
        (goto _label :!via `Reverse`)))))

(fn `UserConstructionScript`)