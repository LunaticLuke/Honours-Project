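; Bedroom cupboards Blueprint with two doors that can each be swung open and closed when something is within that door's detection volume.
; Overlap events on each detect component set a per-door proximity flag, which gates that door's open event.
; A FlipFlop alternates between playing and reversing a timeline, whose output is scaled by a per-door rotation amount to set the door mesh's relative yaw.
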(event `self.Cupboard01_Detect.OnComponentBeginOverlap`
  (params (OverlappedComponent :type "PrimitiveComponent Object Reference") (OtherActor :type "Actor Object Reference") (OtherComp :type "PrimitiveComponent Object Reference") (OtherBodyIndex :type Integer) (bFromSweep :type Boolean) (SweepResult :type "HitResult Structure (by ref)"))
  ;[1 1 1] Near Cupboard01 Detect
  (set `self.NearCupboard01` true))

(event `self.Cupboard01_Detect.OnComponentEndOverlap`
  (params (OverlappedComponent :type "PrimitiveComponent Object Reference") (OtherActor :type "Actor Object Reference") (OtherComp :type "PrimitiveComponent Object Reference") (OtherBodyIndex :type Integer))
  ;[1 1 1] Near Cupboard01 Detect
  (set `self.NearCupboard01` false))

(event `Cupboard01_Open`
  ;[1 1 1] Cupboard01 Open Sequence
  (if (`self.NearCupboard01`)
    (`/Engine/EditorBlueprintResources/StandardMacros.FlipFlop`
      (:`A`
        (bind (_direction _cupboard_rotate_amnt) (`Timeline|Cupboard01 Rotation` :!label _label)
          (:`Update`
            (`SceneComponent.K2_SetRelativeRotation` (`self.SM_Cupboard_Door_01`) (`KismetMathLibrary.MakeRotator` 0.0 0.0 (* _cupboard_rotate_amnt (`self.CupboardDoor01RotAmnt`))) false false))))
      (:`B`
        (goto _label :!via `Reverse`)))))

(event `self.Cupboard02_Detect.OnComponentBeginOverlap`
  (params (OverlappedComponent :type "PrimitiveComponent Object Reference") (OtherActor :type "Actor Object Reference") (OtherComp :type "PrimitiveComponent Object Reference") (OtherBodyIndex :type Integer) (bFromSweep :type Boolean) (SweepResult :type "HitResult Structure (by ref)"))
  ;[1 1 1] Near Cupboard02 Detect
  (set `self.NearCupboard02` true))

(event `self.Cupboard02_Detect.OnComponentEndOverlap`
  (params (OverlappedComponent :type "PrimitiveComponent Object Reference") (OtherActor :type "Actor Object Reference") (OtherComp :type "PrimitiveComponent Object Reference") (OtherBodyIndex :type Integer))
  ;[1 1 1] Near Cupboard02 Detect
  (set `self.NearCupboard02` false))

(event `Cupboard02_Open`
  ;[1 1 1] Cupboard02 Open Sequence
  (if (`self.NearCupboard02`)
    (`/Engine/EditorBlueprintResources/StandardMacros.FlipFlop`
      (:`A`
        (bind (_direction _cupboard02_rotation_amnt) (`Timeline|Cupboard02 Rotation` :!label _label_2)
          (:`Update`
            (`SceneComponent.K2_SetRelativeRotation` (`self.SM_Cupboard_Door_02`) (`KismetMathLibrary.MakeRotator` 0.0 0.0 (* _cupboard02_rotation_amnt (`self.CupboardDoor02RotAmnt`))) false false))))
      (:`B`
        (goto _label_2 :!via `Reverse`)))))

(fn `UserConstructionScript`)