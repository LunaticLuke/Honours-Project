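; A placeable torch Blueprint with a point light and a particle system, whose light flickers during play.
; The construction script applies exposed on/off state, intensity, attenuation radius and colour to the light.
; SetTorchOnOff stores the state and toggles visibility of both light and particles.
; From BeginPlay, a timeline drives intensity between minimum and maximum flicker values, overriding the base intensity while it updates.
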(event `self.ReceiveBeginPlay`
  ;[1 1 1] Torch Flicker Intensity
  (bind (_direction _torchflicker) (`Timeline|TorchFlickerTimeline`)
    (:`Update`
      (`LightComponent.SetIntensity` (`self.TorchPointLight`) (`KismetMathLibrary.Lerp` (`self.TorchFlicker_Min_Intensity`) (`self.TorchFlicker_Max_Intensity`) _torchflicker)))))

(fn `SetTorchOnOff`
  (params (`On / Off` :type Boolean))
  ;[1 1 1] Torch On / Off
  (bind _output_get (set `self.On / Off` `On / Off`))
  (`SceneComponent.SetVisibility` (`self.TorchPointLight`) _output_get false)
  (`SceneComponent.SetVisibility` (`self.TorchParticleSystem`) _output_get false))

(fn `UserConstructionScript`
  ;[1 1 1] Set Torch On / Off - Intensity - Attenuation
  (`self.SetTorchOnOff` (`self.On / Off`))
  (`LightComponent.SetIntensity` (`self.TorchPointLight`) (`self.Torch_Intensity`))
  (`LocalLightComponent.SetAttenuationRadius` (`self.TorchPointLight`) (`self.Torch_Attenuation`))
  (`LightComponent.SetLightColor` (`self.TorchPointLight`) (`self.Torch_Light_Colour`) true))