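; For-loop node Blueprint for VR node building that lets another FunctionNode snap onto it; no loop logic is defined here.
; On AttachmentBox overlap it claims one free FunctionNode and clears its root flag.
; If the player holds this node or its attach parent, the other hand releases and the claimed node snaps to the AttachPoint socket.
; End overlap restores the root flag and frees the slot.
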(event `self.AttachmentBox.OnComponentBeginOverlap`
  (params (OverlappedComponent :type "PrimitiveComponent Object Reference") (OtherActor :type "Actor Object Reference") (OtherComp :type "PrimitiveComponent Object Reference") (OtherBodyIndex :type Integer) (bFromSweep :type Boolean) (SweepResult :type "HitResult Structure (by ref)"))
  (bind _returnvalue (`self.GetAttachParentActor`))
  (if (== (`self.CurrentAttachedNode`) null)
    (bind _asfunction_node (cast `FunctionNode` OtherActor))
    (if (not (`FunctionNode.bAttachedToNode` _asfunction_node))
      (set `FunctionNode.bAttachedToNode` true _asfunction_node)
      (set `self.CurrentAttachedNode` _asfunction_node)
      (set `FunctionNode.RootNode` false _asfunction_node)
      (bind _asbp_vrpawn (cast `/Game/VRTemplate/Blueprints/BP_VRPawn` (`GameplayStatics.GetPlayerPawn` 0)))
      (if (== (`/Game/VRTemplate/Blueprints/BP_VRPawn.HeldComponentLeft` _asbp_vrpawn) (`self.GrabComponent`))
        (set `/Game/VRTemplate/Blueprints/BP_VRPawn.HeldComponentRight` null _asbp_vrpawn)
        (`self.K2_AttachToComponent` _asfunction_node (`self.NodeStaticMesh`) "AttachPoint" "SnapToTarget" "SnapToTarget" "KeepWorld" false :!label _label)
        (set `FunctionNode.CurrentAttachedParent` self (`self.CurrentAttachedNode`))
        (elif (== (`/Game/VRTemplate/Blueprints/BP_VRPawn.HeldComponentRight` _asbp_vrpawn) (`self.GrabComponent`))
          (set `/Game/VRTemplate/Blueprints/BP_VRPawn.HeldComponentLeft` null _asbp_vrpawn)
          (goto _label)
          (elif (== (`/Game/VRTemplate/Blueprints/BP_VRPawn.LeftHeldActor` _asbp_vrpawn) _returnvalue)
            (set `/Game/VRTemplate/Blueprints/BP_VRPawn.HeldComponentRight` null _asbp_vrpawn)
            (goto _label)
            (elif (== (`/Game/VRTemplate/Blueprints/BP_VRPawn.RIghtHeldActor` _asbp_vrpawn) _returnvalue)
              (set `/Game/VRTemplate/Blueprints/BP_VRPawn.HeldComponentLeft` null _asbp_vrpawn)
              (goto _label))))))))

(event `self.AttachmentBox.OnComponentEndOverlap`
  (params (OverlappedComponent :type "PrimitiveComponent Object Reference") (OtherActor :type "Actor Object Reference") (OtherComp :type "PrimitiveComponent Object Reference") (OtherBodyIndex :type Integer))
  (bind _currentattachednode (`self.CurrentAttachedNode`))
  (bind _asfunction_node (cast `FunctionNode` OtherActor))
  (if (== _asfunction_node _currentattachednode)
    (set `FunctionNode.RootNode` true _currentattachednode)
    (set `FunctionNode.bAttachedToNode` false _currentattachednode)
    (set `self.CurrentAttachedNode` null)))

(fn `UserConstructionScript`)