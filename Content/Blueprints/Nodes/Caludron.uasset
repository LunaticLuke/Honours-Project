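; Cauldron actor that takes node actors overlapping its static mesh and feeds them to a Manager as parts of a program.
; An unadded root FunctionNode is registered, then its CurrentAttachedNode chain is walked to register each following node, using AddedToProgram flags against duplicates.
; The Manager then runs the program and the overlapping root node is hidden.
; VariableNodeActors are only added to the program, without running it.
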(event `self.StaticMesh.OnComponentBeginOverlap`
  (params (OverlappedComponent :type "PrimitiveComponent Object Reference") (OtherActor :type "Actor Object Reference") (OtherComp :type "PrimitiveComponent Object Reference") (OtherBodyIndex :type Integer) (bFromSweep :type Boolean) (SweepResult :type "HitResult Structure (by ref)"))
  (bind _manager (`self.Manager`))
  (bind _currentfunctionnode (`self.CurrentFunctionNode`))
  (bind _asfunction_node (cast `FunctionNode` OtherActor)
    (:`then`
      (if (and (`FunctionNode.RootNode` _asfunction_node) (not (`NodeActor.bAddedToProgram` _asfunction_node)))
        (`ProgramManager.AddFunctionToProgram` _manager _asfunction_node)
        (set `NodeActor.bAddedToProgram` true _asfunction_node)
        (set `self.CurrentFunctionNode` (`FunctionNode.CurrentAttachedNode` _asfunction_node))
        (while (!= (`self.CurrentFunctionNode`) null)
          (if (not (`NodeActor.bAddedToProgram` _currentfunctionnode))
            (`ProgramManager.AddFunctionToProgram` (`self.Manager`) _currentfunctionnode)
            (set `NodeActor.bAddedToProgram` true _currentfunctionnode)
            (set `self.CurrentFunctionNode` (`FunctionNode.CurrentAttachedNode` (`self.CurrentFunctionNode`)))))
        (`ProgramManager.RunProgram` _manager)
        (`self.SetActorHiddenInGame` OtherActor true)))
    (:`CastFailed`
      (bind _asvariable_node_actor (cast `VariableNodeActor` OtherActor))
      (`ProgramManager.AddVariableToProgram` _manager _asvariable_node_actor))))

(fn `UserConstructionScript`)