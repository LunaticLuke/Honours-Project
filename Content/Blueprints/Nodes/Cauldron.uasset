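; Cauldron actor that turns dropped node actors into a program, runs it when stirred, and copies it into potions.
; Overlapping function nodes that are chain roots add themselves and their attached nodes to the Manager's program; variable nodes register as variables.
; An overlapping Potion receives the Manager's program data.
; Tick measures the speed of an overlapping Spoon-tagged component's actor and triggers one program run per entry once it moves fast enough.
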(event `self.ReceiveTick`
  (params (DeltaSeconds :type "Float (single-precision)"))
  (bind _spoon (`self.Spoon`))
  (if (and (`KismetSystemLibrary.IsValid` _spoon) (`self.CanStir`))
    (bind _output_get (set `self.Distance` (- (`self.K2_GetActorLocation` _spoon) (`self.LastFramePosition`))))
    (set `self.Velocity` (/ (`KismetMathLibrary.VSize` _output_get) (`GameplayStatics.GetWorldDeltaSeconds`)))
    (set `self.LastFramePosition` (`self.K2_GetActorLocation` (`self.Spoon`)))
    (if (> (`self.Velocity`) 35.0)
      (`ProgramManager.RunProgram` (`self.Manager`))
      (set `self.CanStir` false))))

(event `self.CauldronInterior.OnComponentBeginOverlap`
  (params (OverlappedComponent :type "PrimitiveComponent Object Reference") (OtherActor :type "Actor Object Reference") (OtherComp :type "PrimitiveComponent Object Reference") (OtherBodyIndex :type Integer) (bFromSweep :type Boolean) (SweepResult :type "HitResult Structure (by ref)"))
  (bind _manager (`self.Manager`))
  (bind _currentfunctionnode (`self.CurrentFunctionNode`))
  (bind _manager_2 (`self.Manager`))
  (`|ExecutionSequence`
    (:`then_0`
      (bind _asfunction_node (cast `FunctionNode` OtherActor)
        (:`then`
          (`GameplayStatics.PlaySound2D` "/Game/Audio/object_dropped_in_water_6.object_dropped_in_water_6" 1.0 1.0 0.0 null null)
          (if (and (`FunctionNode.RootNode` _asfunction_node) (not (`NodeActor.bAddedToProgram` _asfunction_node)))
            (`ProgramManager.AddFunctionToProgram` _manager _asfunction_node)
            (set `NodeActor.bAddedToProgram` true _asfunction_node)
            (`KismetSystemLibrary.Delay` 0.25)
            (set `self.CurrentFunctionNode` (`FunctionNode.CurrentAttachedNode` _asfunction_node))
            (while (!= (`self.CurrentFunctionNode`) null)
              (if (not (`NodeActor.bAddedToProgram` _currentfunctionnode))
                (`ProgramManager.AddFunctionToProgram` (`self.Manager`) _currentfunctionnode)
                (set `NodeActor.bAddedToProgram` true _currentfunctionnode)
                (set `self.CurrentFunctionNode` (`FunctionNode.CurrentAttachedNode` (`self.CurrentFunctionNode`)))))
            (`self.SetActorHiddenInGame` OtherActor true)))
        (:`CastFailed`
          (bind _asvariable_node_actor (cast `VariableNodeActor` OtherActor))
          (`ProgramManager.AddVariableToProgram` _manager _asvariable_node_actor)
          (`GameplayStatics.PlaySound2D` "/Game/Audio/object_dropped_in_water_6.object_dropped_in_water_6" 1.0 1.0 0.0 null null))))
    (:`then_1`
      (bind _aspotion (cast `Potion` OtherActor))
      (`KismetSystemLibrary.PrintString` "Hit Potion" true true (struct :`G` 0.66 :`B` 1.0 :`A` 1.0) 5.0)
      (`Potion.SetProgram` _aspotion (`ProgramManager.VariableData` _manager_2) (`ProgramManager.ProgramExecution` _manager_2) (`ProgramManager.ProgramVariables` _manager_2)))
    (:`then_2`
      (if (`ActorComponent.ComponentHasTag` OtherComp "Spoon")
        (set `self.Spoon` OtherActor)
        (set `self.CanStir` true)))))

(event `self.CauldronInterior.OnComponentEndOverlap`
  (params (OverlappedComponent :type "PrimitiveComponent Object Reference") (OtherActor :type "Actor Object Reference") (OtherComp :type "PrimitiveComponent Object Reference") (OtherBodyIndex :type Integer))
  (if (`ActorComponent.ComponentHasTag` OtherComp "Spoon")
    (set `self.Spoon` null)
    (set `self.CanStir` false)))

(fn `UserConstructionScript`)