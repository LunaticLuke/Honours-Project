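; BP_Bedside_Table is a bedside table with a door that swings open and closed.
; A detection component sets a proximity flag on any overlap, with no filter on the overlapping actor, and clears it when overlap ends.
; While that flag is set, the BedsideTableOpen event uses a FlipFlop to alternately play and reverse a timeline that drives the door mesh's relative yaw.
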(event `self.Bedside_Table Detect.OnComponentBeginOverlap`
  (params (OverlappedComponent :type "PrimitiveComponent Object Reference") (OtherActor :type "Actor Object Reference") (OtherComp :type "PrimitiveComponent Object Reference") (OtherBodyIndex :type Integer) (bFromSweep :type Boolean) (SweepResult :type "HitResult Structure (by ref)"))
  ;[1 1 1] Near Bedside Table Detect
  (set `self.NearBedsideTable` true))

(event `self.Bedside_Table Detect.OnComponentEndOverlap`
  (params (OverlappedComponent :type "PrimitiveComponent Object Reference") (OtherActor :type "Actor Object Reference") (OtherComp :type "PrimitiveComponent Object Reference") (OtherBodyIndex :type Integer))
  ;[1 1 1] Near Bedside Table Detect
  (set `self.NearBedsideTable` false))

(event `BedsideTable Open`
  ;[1 1 1] Bedside Table Door Open Sequence
  (if (`self.NearBedsideTable`)
    (`/Engine/EditorBlueprintResources/StandardMacros.FlipFlop`
      (:`A`
        (bind (_direction _bedside_table_roatation_amnt) (`Timeline|Bedside Table Roatation` :!label _label)
          (:`Update`
            (`SceneComponent.K2_SetRelativeRotation` (`self.SM_Bedside_Table_Door`) (`KismetMathLibrary.MakeRotator` 0.0 0.0 _bedside_table_roatation_amnt) false false))))
      (:`B`
        (goto _label :!via `Reverse`)))))

(fn `UserConstructionScript`)