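; BP_Candle_03 is a placeable candle actor with a mesh, a flame particle system and a flickering point light.
; The construction script applies the on/off state, intensity, attenuation radius and light colour from its variables.
; On BeginPlay a timeline drives the light intensity between minimum and maximum flicker values, replacing the set intensity.
; Turning it off hides the light and particles and re-enables the candle mesh's shadow casting.
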(event `self.ReceiveBeginPlay`
  ;[1 1 1] CandleFlicker
  (bind (_direction _candleflicker) (`Timeline|CandleFlickerTimeline`)
    (:`Update`
      (`LightComponent.SetIntensity` (`self.CandllePointLight`) (`KismetMathLibrary.Lerp` (`self.CandleFlicker_Min_Intensity`) (`self.CandleFlicker_Max_Intensity`) _candleflicker)))))

(fn `SetCandleAttenuation`
  (params (Attenuation :type "Float (double-precision)"))
  ;[1 1 1] Set Candle Attenuation Radius
  (bind _output_get (set `self.Candle_Attenuation` Attenuation))
  (`LocalLightComponent.SetAttenuationRadius` (`self.CandllePointLight`) _output_get))

(fn `SetCandleIntensity`
  (params (Intensity :type "Float (double-precision)"))
  ;[1 1 1] Set Candle Overall Intensity
  (bind _output_get (set `self.Candle_Intensity` Intensity))
  (`LightComponent.SetIntensity` (`self.CandllePointLight`) _output_get))

(fn `SetCandleOnOff`
  (params (`On / Off` :type Boolean))
  ;[1 1 1] Candle On / Off
  (bind _output_get (set `self.On / Off` `On / Off`))
  (`SceneComponent.SetVisibility` (`self.CandllePointLight`) _output_get false)
  (`SceneComponent.SetVisibility` (`self.CandleParticleSystem`) _output_get false)
  (`PrimitiveComponent.SetCastShadow` (`self.SM_Candle`) (not _output_get)))

(fn `UserConstructionScript`
  ;[1 1 1] Set Candle On / Off - Intensity - Attenuation
  (`self.SetCandleOnOff` (`self.On / Off`))
  (`LightComponent.SetIntensity` (`self.CandllePointLight`) (`self.Candle_Intensity`))
  (`LocalLightComponent.SetAttenuationRadius` (`self.CandllePointLight`) (`self.Candle_Attenuation`))
  (`LightComponent.SetLightColor` (`self.CandllePointLight`) (`self.Torch_Light_Colour`) true))