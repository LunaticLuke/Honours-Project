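; Fireplace prop Blueprint with a flickering point light, fire particles and a coal mesh.
; The construction script applies the on/off state, light intensity, attenuation, colour and coal visibility from variables.
; SetFireplaceOnOff toggles the light and particle visibility together, leaving the coals separate.
; On BeginPlay, a timeline drives the flicker by lerping light intensity between minimum and maximum values.
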(event `self.ReceiveBeginPlay`
  (bind (_direction _fireplaceflicker_intensity) (`Timeline|FireplaceFlicker Timeline`)
    (:`Update`
      (`LightComponent.SetIntensity` (`self.FireplacePointLight`) (`KismetMathLibrary.Lerp` (`self.FireplaceFlicker_Min_Intensity`) (`self.FireplaceFlicker_Max_Intensity`) _fireplaceflicker_intensity)))))

(fn `SetFireplaceOnOff`
  (params (`On / Off` :type Boolean :default true))
  ;[1 1 1] Fireplace On / Off
  (bind _output_get (set `self.Fireplace On / Off` `On / Off`))
  (`SceneComponent.SetVisibility` (`self.FireplacePointLight`) _output_get false)
  (`SceneComponent.SetVisibility` (`self.FireParticleSystem`) _output_get false))

(fn `UserConstructionScript`
  (`self.SetFireplaceOnOff` (`self.Fireplace On / Off`))
  (`LightComponent.SetIntensity` (`self.FireplacePointLight`) (`self.Fireplace_Intensity`))
  (`LocalLightComponent.SetAttenuationRadius` (`self.FireplacePointLight`) (`self.Fireplace_Attenuation`))
  (`LightComponent.SetLightColor` (`self.FireplacePointLight`) (`self.Fireplace_Colour`) true)
  (`SceneComponent.SetVisibility` (`self.SM_FireplaceCoals`) (`self.FireplaceCoalsVisibility`) false))