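; Six-candle chandelier prop with configurable candle meshes, flame particles and flickering point lights.
; The construction script applies per-candle mesh and flame visibility toggles, plus shared light intensity and attenuation radius.
; On BeginPlay, six separate timelines lerp each light between its own min and max intensity, overriding the shared intensity while they update.
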(event `self.ReceiveBeginPlay`
  ;[1 1 1] Chandelier Candle Flicker
  (`|ExecutionSequence`
    (:`then_0`
      ;;[1 1 1] Candle01 Flicker Intensity
      (bind (_direction _candleflicker) (`Timeline|Candle01 Timeline`)
        (:`Update`
          (`LightComponent.SetIntensity` (`self.Candle01PointLight`) (`KismetMathLibrary.Lerp` (`self.Candle01_Min Intensity`) (`self.Candle01_Max Intensity`) _candleflicker)))))
    (:`then_1`
      ;;[1 1 1] Candle02 Flicker Intensity
      (bind (_direction_2 _candleflicker_2) (`Timeline|Candle02 Timeline`)
        (:`Update`
          (`LightComponent.SetIntensity` (`self.Candle02PointLight`) (`KismetMathLibrary.Lerp` (`self.Candle02_Min Intensity`) (`self.Candle02_Max Intensity`) _candleflicker_2)))))
    (:`then_2`
      ;;[1 1 1] Candle03 Flicker Intensity
      (bind (_direction_3 _candleflicker_3) (`Timeline|Candle03 Timeline`)
        (:`Update`
          (`LightComponent.SetIntensity` (`self.Candle03PointLight`) (`KismetMathLibrary.Lerp` (`self.Candle03_Min Intensity`) (`self.Candle03_Max Intensity`) _candleflicker_3)))))
    (:`then_3`
      ;;[1 1 1] Candle04 Flicker Intensity
      (bind (_direction_4 _candleflicker_4) (`Timeline|Candle04 Timeline`)
        (:`Update`
          (`LightComponent.SetIntensity` (`self.Candle04PointLight`) (`KismetMathLibrary.Lerp` (`self.Candle04_Min Intensity`) (`self.Candle04_Max Intensity`) _candleflicker_4)))))
    (:`then_4`
      ;;[1 1 1] Candle05 Flicker Intensity
      (bind (_direction_5 _candleflicker_5) (`Timeline|Candle05 Timeline`)
        (:`Update`
          (`LightComponent.SetIntensity` (`self.Candle05PointLight`) (`KismetMathLibrary.Lerp` (`self.Candle05_Min Intensity`) (`self.Candle05_Max Intensity`) _candleflicker_5)))))
    (:`then_5`
      ;;[1 1 1] Candle06 Flicker Intensity
      (bind (_direction_6 _candleflicker_6) (`Timeline|Candle06 Timeline`)
        (:`Update`
          (`LightComponent.SetIntensity` (`self.Candle06PointLight`) (`KismetMathLibrary.Lerp` (`self.Candle06_Min Intensity`) (`self.Candle06_Max Intensity`) _candleflicker_6)))))))

(fn `SetCandleFlame01OnOff`
  (params (`On / Off` :type Boolean))
  ;[1 1 1] Set Flame01 On / Off
  (bind _output_get (set `self.Candle01Flame On / Off` `On / Off`))
  (`SceneComponent.SetVisibility` (`self.Candle01PointLight`) _output_get false)
  (`SceneComponent.SetVisibility` (`self.Candle01ParticleSystem`) _output_get false))

(fn `SetCandleFlame02OnOff`
  (params (`On / Off` :type Boolean))
  ;[1 1 1] Set Flame02 On / Off
  (bind _output_get (set `self.Candle02Flame On / Off` `On / Off`))
  (`SceneComponent.SetVisibility` (`self.Candle02PointLight`) _output_get false)
  (`SceneComponent.SetVisibility` (`self.Candle02ParticleSystem`) _output_get false))

(fn `SetCandleFlame03OnOff`
  (params (`On / Off` :type Boolean))
  ;[1 1 1] Set Flame03 On / Off
  (bind _output_get (set `self.Candle03Flame On / Off` `On / Off`))
  (`SceneComponent.SetVisibility` (`self.Candle03PointLight`) _output_get false)
  (`SceneComponent.SetVisibility` (`self.Candle03ParticleSystem`) _output_get false))

(fn `SetCandleFlame04OnOff`
  (params (`On / Off` :type Boolean))
  ;[1 1 1] Set Flame04 On / Off
  (bind _output_get (set `self.Candle04Flame On / Off` `On / Off`))
  (`SceneComponent.SetVisibility` (`self.Candle04PointLight`) _output_get false)
  (`SceneComponent.SetVisibility` (`self.Candle04ParticleSystem`) _output_get false))

(fn `SetCandleFlame05OnOff`
  (params (`On / Off` :type Boolean))
  ;[1 1 1] Set Flame05 On/Off
  (bind _output_get (set `self.Candle05Flame On / Off` `On / Off`))
  (`SceneComponent.SetVisibility` (`self.Candle05PointLight`) _output_get false)
  (`SceneComponent.SetVisibility` (`self.Candle05ParticleSystem`) _output_get false))

(fn `SetCandleFlame06OnOff`
  (params (`On / Off` :type Boolean))
  ;[1 1 1] Set Flame06 On/Off
  (bind _output_get (set `self.Candle06Flame On / Off` `On / Off`))
  (`SceneComponent.SetVisibility` (`self.Candle06PointLight`) _output_get false)
  (`SceneComponent.SetVisibility` (`self.Candle06ParticleSystem`) _output_get false))

(fn `SetCandleMesh01OnOff`
  (params (`On / Off` :type Boolean))
  ;[1 1 1] Set Candle01Mesh On/Off
  (bind _output_get (set `self.Candle01Mesh On / Off` `On / Off`))
  (`SceneComponent.SetVisibility` (`self.SM_Candle01`) _output_get false))

(fn `SetCandleMesh02OnOff`
  (params (`On / Off` :type Boolean))
  ;[1 1 1] Set Candle02Mesh On/Off
  (bind _output_get (set `self.Candle02Mesh On / Off` `On / Off`))
  (`SceneComponent.SetVisibility` (`self.SM_Candle02`) _output_get false))

(fn `SetCandleMesh03OnOff`
  (params (`On / Off` :type Boolean))
  ;[1 1 1] Set Candle03Mesh On/Off
  (bind _output_get (set `self.Candle03Mesh On / Off` `On / Off`))
  (`SceneComponent.SetVisibility` (`self.SM_Candle03`) _output_get false))

(fn `SetCandleMesh04OnOff`
  (params (`On / Off` :type Boolean))
  ;[1 1 1] Set Candle04Mesh On/Off
  (bind _output_get (set `self.Candle04Mesh On / Off` `On / Off`))
  (`SceneComponent.SetVisibility` (`self.SM_Candle04`) _output_get false))

(fn `SetCandleMesh05OnOff`
  (params (`On / Off` :type Boolean))
  ;[1 1 1] Set Candle05Mesh On/Off
  (bind _output_get (set `self.Candle05Mesh On / Off` `On / Off`))
  (`SceneComponent.SetVisibility` (`self.SM_Candle05`) _output_get false))

(fn `SetCandleMesh06OnOff`
  (params (`On / Off` :type Boolean))
  ;[1 1 1] Set Mesh06 On/Off
  (bind _output_get (set `self.Candle06Mesh On / Off` `On / Off`))
  (`SceneComponent.SetVisibility` (`self.SM_Candle06`) _output_get false))

(fn `SetChandelierAttenuation`
  (params (Attenuation :type "Float (double-precision)"))
  ;[1 1 1] Set Chandelier Attenuation Radius
  (bind _output_get (set `self.Chandelier_Attenuation` Attenuation))
  (`LocalLightComponent.SetAttenuationRadius` (`self.Candle02PointLight`) _output_get)
  (`LocalLightComponent.SetAttenuationRadius` (`self.Candle01PointLight`) _output_get)
  (`LocalLightComponent.SetAttenuationRadius` (`self.Candle03PointLight`) _output_get)
  (`LocalLightComponent.SetAttenuationRadius` (`self.Candle04PointLight`) _output_get)
  (`LocalLightComponent.SetAttenuationRadius` (`self.Candle05PointLight`) _output_get)
  (`LocalLightComponent.SetAttenuationRadius` (`self.Candle06PointLight`) _output_get))

(fn `SetChandelierIntensity`
  (params (Intensity :type "Float (double-precision)"))
  ;[1 1 1] Set Chandelier Intensity
  (`LightComponent.SetIntensity` (`self.Candle01PointLight`) Intensity)
  (`LightComponent.SetIntensity` (`self.Candle02PointLight`) Intensity)
  (`LightComponent.SetIntensity` (`self.Candle04PointLight`) Intensity)
  (`LightComponent.SetIntensity` (`self.Candle05PointLight`) Intensity)
  (`LightComponent.SetIntensity` (`self.Candle06PointLight`) Intensity)
  (`LightComponent.SetIntensity` (`self.Candle03PointLight`) Intensity))

(fn `UserConstructionScript`
  ;[1 1 1] Chandelier Candle Mesh/Lights/ParticleSystems -  On / Off
  (`self.SetCandleFlame01OnOff` (`self.Candle01Flame On / Off`))
  (`self.SetCandleMesh01OnOff` (`self.Candle01Mesh On / Off`))
  (`self.SetCandleFlame02OnOff` (`self.Candle02Flame On / Off`))
  (`self.SetCandleMesh02OnOff` (`self.Candle02Mesh On / Off`))
  (`self.SetCandleFlame03OnOff` (`self.Candle03Flame On / Off`))
  (`self.SetCandleMesh03OnOff` (`self.Candle03Mesh On / Off`))
  (`self.SetCandleFlame04OnOff` (`self.Candle04Flame On / Off`))
  (`self.SetCandleMesh04OnOff` (`self.Candle04Mesh On / Off`))
  (`self.SetCandleFlame05OnOff` (`self.Candle05Flame On / Off`))
  (`self.SetCandleMesh05OnOff` (`self.Candle05Mesh On / Off`))
  (`self.SetCandleFlame06OnOff` (`self.Candle06Flame On / Off`))
  (`self.SetCandleMesh06OnOff` (`self.Candle06Mesh On / Off`))
  (`self.SetChandelierIntensity` (`self.Chandelier Intensity`))
  (`self.SetChandelierAttenuation` (`self.Chandelier_Attenuation`)))