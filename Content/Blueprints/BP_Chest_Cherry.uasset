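; BP_Chest_Cherry is a cherry chest that opens and closes its lid when triggered while something is within its detection area.
; Overlap events on the detection component set a NearChest flag, which gates the Chest_Cherry_Open event.
; A FlipFlop alternates between playing and reversing a timeline, whose curve value scaled by LidRotationAmount drives the lid mesh's relative roll.
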(event `self.Chest_Cherry_Detection.OnComponentBeginOverlap`
  (params (OverlappedComponent :type "PrimitiveComponent Object Reference") (OtherActor :type "Actor Object Reference") (OtherComp :type "PrimitiveComponent Object Reference") (OtherBodyIndex :type Integer) (bFromSweep :type Boolean) (SweepResult :type "HitResult Structure (by ref)"))
  ;[1 1 1] Chest Detection
  (set `self.NearChest` true))

(event `self.Chest_Cherry_Detection.OnComponentEndOverlap`
  (params (OverlappedComponent :type "PrimitiveComponent Object Reference") (OtherActor :type "Actor Object Reference") (OtherComp :type "PrimitiveComponent Object Reference") (OtherBodyIndex :type Integer))
  ;[1 1 1] Chest Detection
  (set `self.NearChest` false))

(event `Chest_Cherry_Open`
  ;[1 1 1] Chest Open Sequence
  (if (`self.NearChest`)
    (`/Engine/EditorBlueprintResources/StandardMacros.FlipFlop`
      (:`A`
        (bind (_direction _lidrotation) (`Timeline|ChestOpenAmountTimeline` :!label _label)
          (:`Update`
            (`SceneComponent.K2_SetRelativeRotation` (`self.SM_Chest_Cherry_Lid`) (`KismetMathLibrary.MakeRotator` (* _lidrotation (`self.LidRotationAmount`))) false false))))
      (:`B`
        (goto _label :!via `Reverse`)))))

(fn `UserConstructionScript`)