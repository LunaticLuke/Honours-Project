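; Dressing table Blueprint with two drawers that slide open and closed independently.
; Each drawer has a detection component whose begin and end overlaps set its Near flag, without filtering the overlapping actor.
; Drawer01Open and Drawer02Open check that flag, then use a FlipFlop to alternately play and reverse a timeline that drives the drawer's relative location.
; Nothing in this graph calls those two open events.
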(event `self.Drawer01_Detection.OnComponentBeginOverlap`
  (params (OverlappedComponent :type "PrimitiveComponent Object Reference") (OtherActor :type "Actor Object Reference") (OtherComp :type "PrimitiveComponent Object Reference") (OtherBodyIndex :type Integer) (bFromSweep :type Boolean) (SweepResult :type "HitResult Structure (by ref)"))
  ;[1 1 1] Near Drawer01 Detection
  (set `self.NearDrawer01` true))

(event `self.Drawer01_Detection.OnComponentEndOverlap`
  (params (OverlappedComponent :type "PrimitiveComponent Object Reference") (OtherActor :type "Actor Object Reference") (OtherComp :type "PrimitiveComponent Object Reference") (OtherBodyIndex :type Integer))
  ;[1 1 1] Near Drawer01 Detection
  (set `self.NearDrawer01` false))

(event `Drawer01Open`
  ;[1 1 1] Drawer01Open
  (if (`self.NearDrawer01`)
    (`/Engine/EditorBlueprintResources/StandardMacros.FlipFlop`
      (:`A`
        (bind (_direction _drawer01translate) (`Timeline|Drawer01_Translation_Amount` :!label _label)
          (:`Update`
            (`SceneComponent.K2_SetRelativeTransform` (`self.Drawer01`) (`KismetMathLibrary.MakeTransform` _drawer01translate) false false))))
      (:`B`
        (goto _label :!via `Reverse`)))))

(event `self.Drawer02_Detection.OnComponentBeginOverlap`
  (params (OverlappedComponent :type "PrimitiveComponent Object Reference") (OtherActor :type "Actor Object Reference") (OtherComp :type "PrimitiveComponent Object Reference") (OtherBodyIndex :type Integer) (bFromSweep :type Boolean) (SweepResult :type "HitResult Structure (by ref)"))
  ;[1 1 1] Drawer02 Detection
  (set `self.NearDrawer02` true))

(event `self.Drawer02_Detection.OnComponentEndOverlap`
  (params (OverlappedComponent :type "PrimitiveComponent Object Reference") (OtherActor :type "Actor Object Reference") (OtherComp :type "PrimitiveComponent Object Reference") (OtherBodyIndex :type Integer))
  ;[1 1 1] Drawer02 Detection
  (set `self.NearDrawer02` false))

(event `Drawer02Open`
  ;[1 1 1] Drawer02Open
  (if (`self.NearDrawer02`)
    (`/Engine/EditorBlueprintResources/StandardMacros.FlipFlop`
      (:`A`
        (bind (_direction _drawer02_translate) (`Timeline|Drawer02_Translation_Amount` :!label _label_2)
          (:`Update`
            (`SceneComponent.K2_SetRelativeTransform` (`self.Drawer02`) (`KismetMathLibrary.MakeTransform` _drawer02_translate) false false))))
      (:`B`
        (goto _label_2 :!via `Reverse`)))))

(fn `UserConstructionScript`)